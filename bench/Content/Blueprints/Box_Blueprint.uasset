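; Box trigger actor that reports to ThirdPersonGameMode when its collision component is overlapped, then removes itself.
; BeginPlay creates Task_Popup and Task_UI widgets without displaying them and caches the game mode.
; Any overlap, with no actor check, sets Boxactive on the game mode, calls Triggered and destroys the box.
; The timed task-widget sequence, including its Taskfunction call to show Task_UI, is disconnected and never runs.
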(event `self.ReceiveBeginPlay`
  (bind _returnvalue (`|CreateWidget` "/Game/HUD/Task_Popup.Task_Popup_C"))
  (set `self.taskpopup` _returnvalue)
  (bind _returnvalue_2 (`|CreateWidget` "/Game/HUD/Task_UI.Task_UI_C"))
  (set `self.taskui` _returnvalue_2)
  (bind _asthird_person_game_mode (cast `/Game/Blueprints/ThirdPersonGameMode` (`GameplayStatics.GetGameMode`)))
  (set `self.game object` _asthird_person_game_mode))

(event `self.CollisionComponent.OnComponentBeginOverlap`
  (params (OverlappedComponent :type "PrimitiveComponent Object Reference") (OtherActor :type "Actor Object Reference") (OtherComp :type "PrimitiveComponent Object Reference") (OtherBodyIndex :type Integer) (bFromSweep :type Boolean) (SweepResult :type "HitResult Structure (by ref)"))
  (set `/Game/Blueprints/ThirdPersonGameMode.boxactive` true (`self.game object`))
  (`/Game/Blueprints/ThirdPersonGameMode.triggered` (`self.game object`))
  (`self.K2_DestroyActor`))

(fn `Taskfunction`
  (bind _returnvalue (`|CreateWidget` "/Game/HUD/Task_UI.Task_UI_C"))
  (`UserWidget.AddToViewport` _returnvalue 0))

(fn `UserConstructionScript`)